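; Player controller for the lobby menu, handling UI-only input, the lobby widget and the player's saved profile.
; InitialSetup loads the profile from a local save slot, creating a default save if none exists, then passes it to ServerUpdateLobby.
; That event stores the profile and tells ELOLMenuMode_BP to update the lobby.
; UpdatePlayerNames refreshes the names shown in the lobby widget from the supplied profiles.
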(event Custom|CreateLobbyMenu
  (CallFunction|UIShowLobbyMenu))

(event Custom|InitialSetup
  (CallFunction|LoadSavedProfile)
  (CallFunction|ServerUpdateLobby (Variables|Default|GetPlayerProfileInformation)))

(event Custom|UpdatePlayerNames
  (params (PlayerProfiles :type Array%20of%20S%20Player%20Profile%20Structures))
  (bind _lobbymenu (Variables|Default|GetLobbyMenu))
  (Utilities|IsValid _lobbymenu
    (:Is%20Valid
      (Default|ClearPlayerNames _lobbymenu)
      (Default|UpdatePlayerNames _lobbymenu PlayerProfiles))))

(event Custom|ServerUpdateLobby
  (params (PlayerProfile :type S%20Player%20Profile%20Structure))
  (Variables|Default|SetPlayerProfileInformation PlayerProfile)
  (bind _aselolmenu_mode_bp (Utilities|Casting|CastToELOLMenuMode_BP (Game|GetGameMode)))
  (Default|UpdateLobby _aselolmenu_mode_bp true))

(event EventBeginPlay
  (if (Pawn|IsLocalController)
    (Variables|Default|SetbShowMouseCursor true)
    (Input|SetInputModeUIOnly self 0 "DoNotLock" false)))

(fn ConstructionScript)

(fn UIShowLobbyMenu
  (Utilities|IsValid (Variables|Default|GetLobbyMenu)
    (:Is%20Valid
      _)
    (:Is%20Not%20Valid
      (bind _returnvalue (UserInterface|CreateWidget "/Game/Widgets/ELOLLobbyMenu.ELOLLobbyMenu_C" self))
      (Variables|Default|SetLobbyMenu _returnvalue)))
  (UserInterface|Viewport|AddtoViewport (Variables|Default|GetLobbyMenu) 0)
  (return))

(fn LoadSavedProfile
  (bind _returnvalue (SaveGame|DoesSaveGameExist (LocalVariables|GetLocalSlotName)))
  (if _returnvalue
    _
    (else
      (bind _returnvalue_2 (SaveGame|CreateSaveGameObject "/Game/SaveData/SG_PlayerProfile.SG_PlayerProfile_C"))
      (SaveGame|SaveGametoSlot _returnvalue_2 (LocalVariables|GetLocalSlotName))))
  (bind _returnvalue_3 (SaveGame|LoadGamefromSlot (LocalVariables|GetLocalSlotName)))
  (bind _assg_player_profile (Utilities|Casting|CastToSG_PlayerProfile _returnvalue_3))
  (Variables|Default|SetPlayerProfileInformation (Variables|/Game/SaveData/SG_PlayerProfile.SG_PlayerProfile_C|GetPlayerProfile _assg_player_profile))
  (return))