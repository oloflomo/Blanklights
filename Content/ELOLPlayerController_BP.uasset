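; Player controller for the ELOL game that handles cursor, respawn and exit-menu input.
; On BeginPlay the local controller switches to game-only input and hides the mouse cursor, and InputSwap toggles cursor visibility.
; The reset action calls a custom event that asks the WarpMap game mode to respawn players.
; The 9 key creates and shows a MapExitMenu widget.
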(event Custom|CustomEvent
  (bind _asmy_elolbase_mode_warp_map (Utilities|Casting|CastToMyELOLBaseMode_WarpMap (Game|GetGameMode)))
  (Default|RespawnPlayers _asmy_elolbase_mode_warp_map))

(event EventBeginPlay
  (if (Pawn|IsLocalPlayerController)
    (Input|SetInputModeGameOnly self false)
    (Variables|Default|SetbShowMouseCursor false)))

(event Input|ActionEvents|InputActionInputSwap
  (params (Key :type Key%20Structure :default "None"))
  (:Pressed
    (if (Variables|Default|GetbShowMouseCursor)
      (Variables|Default|SetbShowMouseCursor false)
      (else
        (Variables|Default|SetbShowMouseCursor true)))))

(event Input|ActionEvents|InputActionreset
  (params (Key :type Key%20Structure :default "None"))
  (:Pressed
    (CallFunction|CustomEvent)))

(event Input|KeyboardEvents|9
  (params (Key :type Key%20Structure :default "None"))
  (:Pressed
    (bind _returnvalue (UserInterface|CreateWidget "/Game/Widgets/MapExitMenu.MapExitMenu_C" self))
    (UserInterface|Viewport|AddtoViewport _returnvalue 0)))

(fn ConstructionScript)