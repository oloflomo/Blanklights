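; MainHUD_BP is a HUD Blueprint that shows and hides three UMG widgets: the map exit menu, the ship interface and the map select screen.
; Each Show event creates a fresh widget for the owning player controller, stores it in a variable and adds it to the viewport.
; The matching Hide events remove the stored widget from its parent, with no validity or duplicate checks.
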(event Custom|ShowMapSelect
  (bind _returnvalue (UserInterface|CreateWidget "/Game/Widgets/MapSelectWIdget.MapSelectWIdget_C" (Game|Player|GetOwningPlayerController)))
  (bind _output_get (Variables|Default|SetMapSelect _returnvalue))
  (UserInterface|Viewport|AddtoViewport _output_get 0))

(event Custom|ShowShipInterface
  (bind _returnvalue (UserInterface|CreateWidget "/Game/Widgets/ShipInterface.ShipInterface_C" (Game|Player|GetOwningPlayerController)))
  (bind _output_get (Variables|Default|SetShipInterface _returnvalue))
  (UserInterface|Viewport|AddtoViewport _output_get 0))

(event Custom|HideShipInterface
  (Widget|RemovefromParent (Variables|Default|GetShipInterface)))

(event Custom|HideMapSelect
  (Widget|RemovefromParent (Variables|Default|GetMapSelect)))

(event Custom|ShowExitMenu
  (bind _returnvalue (UserInterface|CreateWidget "/Game/Widgets/MapExitMenu.MapExitMenu_C" (Game|Player|GetOwningPlayerController)))
  (bind _output_get (Variables|Default|SetExitMenu _returnvalue))
  (UserInterface|Viewport|AddtoViewport _output_get 0))

(event Custom|HideExitMenu
  (Widget|RemovefromParent (Variables|Default|GetExitMenu)))

(fn ConstructionScript)