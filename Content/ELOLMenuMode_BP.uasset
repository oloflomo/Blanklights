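; Menu game mode that manages players joining the lobby and keeps their profile lists in sync.
; When a new player starts on the Lobby Map, it records their ELOLMenuController_BP, then has it create the lobby menu and run initial setup.
; UpdateLobby, when flagged for player names, rebuilds the profile array from all connected controllers and pushes it back to each one.
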(event Custom|UpdateLobby
  (params (PlayerNames :type Boolean))
  (if PlayerNames
    (Utilities|Array|Clear (Variables|Default|GetAllPlayerProfiles))
    (for _array_element (Variables|Default|GetAllConnectedPlayers)
      (Utilities|Array|Add (Variables|Default|GetAllPlayerProfiles) (Variables|/Game/ELOLMenuController_BP.ELOLMenuController_BP_C|GetPlayerProfileInformation _array_element)))
    (for _array_element_2 (Variables|Default|GetAllConnectedPlayers)
      (if PlayerNames
        (Default|UpdatePlayerNames _array_element_2 (Variables|Default|GetAllPlayerProfiles))))))

(event EventHandleStartingNewPlayer
  (params (NewPlayer :type Player%20Controller%20Object%20Reference))
  (bind _returnvalue (Game|GetCurrentLevelName true))
  (switch string _returnvalue
    (:LobbyMap
      (bind _aselolmenu_controller_bp (Utilities|Casting|CastToELOLMenuController_BP NewPlayer))
      (Utilities|Array|Add (Variables|Default|GetAllConnectedPlayers) _aselolmenu_controller_bp)
      (Default|CreateLobbyMenu _aselolmenu_controller_bp)
      (Default|InitialSetup _aselolmenu_controller_bp))))

(fn ConstructionScript)