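; WidgetPawn_BP is a pawn that shows the mouse cursor on BeginPlay and fires a debug line trace from its camera.
; Both press and release of the Fire input run the same Camera-channel trace, projected far along the camera's forward vector from a start offset in world space.
; The trace is drawn for a duration, but its result is unused.
; Disconnected nodes hold an unused mouse-position-based trace calculation.
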(event EventBeginPlay
  (Variables|/Script/Engine.PlayerController|SetbShowMouseCursor (Game|GetPlayerController 0) true))

(event Input|ActionEvents|InputActionFire
  (params (Key :type Key%20Structure :default "None"))
  (bind _camera (Variables|Default|GetCamera))
  (bind _returnvalue (Transformation|GetWorldLocation _camera))
  (bind _returnvalue_2 (Math|Vector|GetForwardVector _camera))
  (bind (_x _y _z) (Math|Vector|BreakVector _returnvalue_2))
  (bind (_x_2 _y_2 _z_2) (Math|Vector|BreakVector _returnvalue))
  (:Pressed
    (Collision|LineTraceByChannel (Math|Vector|MakeVector (+ _x_2 1e+02) _y_2 (+ _z_2 1.0)) (+ _returnvalue (Math|Vector|MakeVector (* _x 1e+04) (* _y 1e+04) (* _z 1e+04))) "TraceTypeQuery2" false 0 "ForDuration" :!label _label))
  (:Released
    (goto _label)))

(fn ConstructionScript)